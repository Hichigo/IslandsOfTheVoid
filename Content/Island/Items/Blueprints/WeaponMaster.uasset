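; WeaponMaster is a world item actor that rolls a random equipment identity and can be picked up by the player.
; On BeginPlay it links itself to its name-label widget and fills its Info struct with a placeholder cube and two independently randomized picks: slot label and enum value.
; PickupBtn checks that the player character is in range, sends Info to the player controller via PickupMessage, then destroys the actor.
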(event Custom|PickupBtn
  (if (<= (Transformation|GetDistanceTo (Game|GetPlayerCharacter 0)) 3e+02)
    (Class|HeroInteract|Pickup(Message) (Game|GetPlayerController 0) (Variables|Default|GetInfo))
    (Actor|DestroyActor)))

(event EventBeginPlay
  (bind _returnvalue (Math|Random|RandomInteger 8))
  (bind _asname_item_widget (Utilities|Casting|CastToNameItemWidget (UserInterface|GetUserWidgetObject (Variables|Default|GetPickupBtnName))))
  (Variables|/Game/Island/Items/UMG/NameItemWidget.NameItemWidget_C|Setweapon _asname_item_widget self)
  (Variables|Default|SetInfo (Utilities|Struct|MakeStoredItem "NewEnumerator0" false "(Name_2_F26A6ED24888233AF68DEA9E5AF095E8=\"\",TypeWeapon_37_DB66544E47C532EFA02C0CB05E465FE3=NewEnumerator0,Hands_38_9C77EACB41FBA76BCFBCEDAC201B37E9=NewEnumerator0,DmageMin_9_5658F03149A138AE4E98FDAA3603F18D=0.000000,DamageMax_11_090FBE2C4151A256B7D5939C428681D4=0.000000,AttackSpeed_13_337DA3544B1C4B5C1B38FB9E72CB70AF=0.000000,ChanceCrit_15_C55814A04BCECDAA0C1633936AC54CAA=0.000000,PowerCrit_17_66ABDDD64B276BE45DC100B0ED3D3180=0.000000,Weight_19_9C707D9E41D360B0DBBA1A8FFF2E7017=0.000000,StrengthPercent_22_DB77AA0345BAD9D46C7644AB2FB7D398=0.000000,AgilityPercent_24_B2BEC0A44D9C65598FABAFB1E8EBFBF7=0.000000,IntelligencePercent_26_83338F5A45E2D974F3E05DA3C328D67C=0.000000,Description_29_65DAA21B4B3AD145E76CD5870452BACE=\"\",Price_33_34E5463B4A9DB5651931B48417E38162=0)" "(Name_12_F26A6ED24888233AF68DEA9E5AF095E8=\"\",TypeArmor_38_721674644E225E21A56B60B15C7EFDB1=NewEnumerator0,Defence_28_5B76DCB24F411514425119B78F4680E2=0.000000,ResistFire_29_3C9E37EF4C444F59B0B0ECB777D7E19A=0.000000,ResistCold_30_D8D6449647ABE04EBAB7BAB729E58D2B=0.000000,ResistLightning_31_43E14B6342CB5EFF1896449FF05BCAFA=0.000000,ResistPotion_32_6D12A911447506D7DF39A7BB091AA45A=0.000000,Weight_33_54E34BC144C5A6433636B49732E6086B=0.000000,StrengthPercent_34_41CFBC054E6057C947D9FDB2336F1EEC=0.000000,AgilityPercent_35_F72E493242BAC7613C1CF685E67F0E7D=0.000000,IntelligencePercent_36_A29A496642706C724AC8C081D2B29A2A=0.000000,Description_26_12D9A43A4ADD283D3AC4A1B4AF288683=\"\",Price_39_A48EF3DA4AB0D212ECBC7881C7A9862F=0)" "(Name_18_F26A6ED24888233AF68DEA9E5AF095E8=\"\",TypePotion_19_A3DBBC8645AE419DEF457AACD732A643=NewEnumerator0,Restore_16_4CE0C08149A06ACA1A1E9B92F23396F7=0.000000,Weight_15_DBF9A0984DB9C6073E9BF2A4F4426567=0.000000,Description_14_DA69FE6243BF7F6C834E8BBCA9D9C0D9=\"\",Price_13_F148E80B46D94F59272BD8A9D9123F6E=0)" "(Name_13_F26A6ED24888233AF68DEA9E5AF095E8=\"\",TypeCraft_15_64A129804AC6CE3A981ED69B3F714140=NewEnumerator0,Weight_14_7A4221224A9F0457420275893506F08E=0.000000,Description_12_16F7A14045282929E6BB8081CD52BB0E=\"\",Price_11_091A4DE14760B219F10BA2B1D8CB6BCA=0)" "(Name_9_F26A6ED24888233AF68DEA9E5AF095E8=\"\",Weight_11_C343314544A235F3FD044BB4338BEACC=0.000000,Description_10_2FB2568842F0862BFE6101906145ED9C=\"\",Price_8_75E5859C45311762ABBF22A1015643ED=0)" "/Game/Geometry/Meshes/1M_Cube.1M_Cube" (Utilities|Select :Index _returnvalue :Option%200 "/Game/Island/Items/UI_Textures/helm.helm" :Option%201 "/Game/Island/Items/UI_Textures/neck.neck" :Option%202 "/Game/Island/Items/UI_Textures/sword.sword" :Option%203 "/Game/Island/Items/UI_Textures/ring.ring" :Option%204 "/Game/Island/Items/UI_Textures/shield.shield" :Option%205 "/Game/Island/Items/UI_Textures/boots.boots" :Option%206 "/Game/Island/Items/UI_Textures/Pants.Pants" :Option%207 "/Game/Island/Items/UI_Textures/gloves.gloves") (Utilities|Select :Index _returnvalue :Option%200 "NewEnumerator0" :Option%201 "NewEnumerator5" :Option%202 "NewEnumerator11" :Option%203 "NewEnumerator9" :Option%204 "NewEnumerator10" :Option%205 "NewEnumerator4" :Option%206 "NewEnumerator3" :Option%207 "NewEnumerator7"))))

(fn ConstructionScript
  (|CallParentFunction))