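; HeroPC is the Hero's player controller, handling item pickup, inventory, sprint and a few test key bindings.
; Pickup stores items in the first slot found by InventoryEquipStatManagerComponent, printing a warning when full, while I opens the inventory through InventoryComponent.
; Left Shift toggles the manager's sprint flag and walk speed, and StopSprinting reuses the release path.
; Hardcoded C and V keys grant a large experience boost and play a sword-slash montage.
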(event Custom|StopSprinting
  (Variables|/Game/Island/Components/Manager/InventoryEquipStatManagerComponent.InventoryEquipStatManagerComponent_C|SetSprinting (Variables|Default|GetInventoryEquipStatManagerComponent) false)
  (Variables|/Script/Engine.CharacterMovementComponent|SetMaxWalkSpeed (Variables|/Script/Engine.Character|GetCharacterMovement (Variables|Default|GetCharacterRef)) 4.5e+02))

(event EventPickup
  (params (Info :type Stored%20Item%20Structure))
  (bind (_emptyindex _isfind) (Default|FindEmptySlot (Variables|Default|GetInventoryEquipStatManagerComponent)))
  (if _isfind
    (Default|PutintheSlot (Variables|Default|GetInventoryEquipStatManagerComponent) _emptyindex Info)
    (else
      (Development|PrintString "*** INVETORY IS FULL ***" true true "(R=1.000000,G=0.000000,B=0.000000,A=1.000000)"))))

(event EventBeginPlay
  (bind _ashero (Utilities|Casting|CastToHero (Game|GetPlayerCharacter 0)))
  (Variables|Default|SetCharacterRef _ashero))

(event Input|KeyboardEvents|I
  (params (Key :type Key%20Structure :default "AnyKey"))
  ;[1 1 1] Open inventory
  (:Pressed
    (Default|OpenInventory (Variables|Default|GetInventoryComponent))))

(event Input|KeyboardEvents|LeftShift
  (params (Key :type Key%20Structure :default "AnyKey"))
  (bind _inventoryequipstatmanagercomponent (Variables|Default|GetInventoryEquipStatManagerComponent))
  (bind _characterref (Variables|Default|GetCharacterRef))
  (bind _charactermovement (Variables|/Script/Engine.Character|GetCharacterMovement _characterref))
  (:Pressed
    (Variables|/Game/Island/Components/Manager/InventoryEquipStatManagerComponent.InventoryEquipStatManagerComponent_C|SetSprinting _inventoryequipstatmanagercomponent true)
    (Variables|/Script/Engine.CharacterMovementComponent|SetMaxWalkSpeed _charactermovement 6e+02))
  (:Released
    (Variables|/Game/Island/Components/Manager/InventoryEquipStatManagerComponent.InventoryEquipStatManagerComponent_C|SetSprinting _inventoryequipstatmanagercomponent false)
    (Variables|/Script/Engine.CharacterMovementComponent|SetMaxWalkSpeed _charactermovement 4.5e+02)))

(event Input|KeyboardEvents|C
  (params (Key :type Key%20Structure :default "AnyKey"))
  (:Pressed
    (Default|AddExp (Variables|Default|GetInventoryEquipStatManagerComponent) 2e+06)))

(event Input|KeyboardEvents|V
  (params (Key :type Key%20Structure :default "AnyKey"))
  (:Pressed
    (Animation|PlayAnimMontage (Variables|Default|GetCharacterRef) "/Game/Island/Character/Animations/sword_and_shield_slash4_Montage.sword_and_shield_slash4_Montage" 1.0 "None")))

(fn ConstructionScript)