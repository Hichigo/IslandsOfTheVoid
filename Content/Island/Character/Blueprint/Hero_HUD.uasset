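; Hero HUD Blueprint that creates the Bars widget and places it in the top-left area of the viewport on BeginPlay.
; After a zero-length delay, it asks the HeroPC controller's InventoryEquipStatManagerComponent to refresh the health, endurance, experience and level displays.
; It prints an error if the player controller is not a HeroPC.
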(event EventBeginPlay
  (bind _returnvalue (UserInterface|CreateWidget "/Game/Island/Components/Stats/UMG/Bars.Bars_C" (Game|GetPlayerController 0)))
  (bind _output_get (Variables|Default|SetBars _returnvalue))
  (UserInterface|Viewport|AddtoViewport _output_get 0)
  (Class|UserWidget|SetPositioninViewport _output_get "(X=50.000000,Y=50.000000)" true)
  (bind _ashero_pc (Utilities|Casting|CastToHeroPC (Game|GetPlayerController 0))
    (:then
      (Utilities|FlowControl|Delay 0.0)
      (Default|UpdateHealthBar (Variables|/Game/Island/Character/Blueprint/HeroPC.HeroPC_C|GetInventoryEquipStatManagerComponent _ashero_pc))
      (Default|UpdateEnduranceBar (Variables|/Game/Island/Character/Blueprint/HeroPC.HeroPC_C|GetInventoryEquipStatManagerComponent _ashero_pc))
      (Default|UpdateExpBar (Variables|/Game/Island/Character/Blueprint/HeroPC.HeroPC_C|GetInventoryEquipStatManagerComponent _ashero_pc))
      (Default|UpdateLvl (Variables|/Game/Island/Character/Blueprint/HeroPC.HeroPC_C|GetInventoryEquipStatManagerComponent _ashero_pc)))
    (:CastFailed
      (Development|PrintString "*** fail cast to controller in HUD ***" true true "(R=1.000000,G=0.000000,B=0.000000,A=1.000000)" 1e+01))))

(fn ConstructionScript)