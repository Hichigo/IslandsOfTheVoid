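; Hero is the player character Blueprint for the Island game, handling top-down style movement and inventory interaction.
; MoveForward and MoveRight axes add movement along fixed world X and Y directions, independent of the controller rotation.
; A Pickup event asks the inventory component for an empty slot and stores weapon-type items there.
; The I key opens the inventory through the same component.
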(event EventPickup
  (params (TypeItem :type TypeItem%20Enum) (Weapon :type Weapon%20Structure))
  (bind _emptyindex (Default|FindEmptySlot (Variables|Default|GetInventoryComp)))
  (switch Utilities|FlowControl|Switch|SwitchonTypeItem TypeItem
    (:NewEnumerator0
      (Default|PutintheSlot (Variables|Default|GetInventoryComp) _emptyindex TypeItem Weapon))))

(event Input|AxisEvents|InputAxisMoveForward
  (params (AxisValue :type Float%20%28single-precision%29))
  ;[1 1 1] Movement
  (Pawn|Input|AddMovementInput "1.000000, 0, 0" AxisValue false))

(event Input|AxisEvents|InputAxisMoveRight
  (params (AxisValue :type Float%20%28single-precision%29))
  ;[1 1 1] Movement
  (Pawn|Input|AddMovementInput "0.000000,1.000000, 0" AxisValue false))

(event Input|KeyboardEvents|I
  (params (Key :type Key%20Structure :default "AnyKey"))
  ;[1 1 1] Open inventory
  (:Pressed
    (Default|OpenInventory (Variables|Default|GetInventoryComp))))

(fn ConstructionScript)